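; BP_Spawner is a pooled spawner for BP_Note actors.
; On BeginPlay it spawns a set number of notes at its own transform, disables their mesh collision, binds their destruction event and stores them in NotePool.
; Each Spawn event activates the note at NoteIndex if valid, then advances the index, wrapping to reuse the pool in round-robin order.
; OnNoteDestroyed only sets the spawner's location to its current location.
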(event `self.ReceiveBeginPlay`
  (`self.SpawnNotes`))

(event `OnNoteDestroyed`
  (params (Notes :type "/Game/Notes/BP_Note Object Reference"))
  (`self.K2_SetActorLocation` (`self.K2_GetActorLocation`)))

(event `Spawn`
  (bind _notepool (`self.NotePool`))
  (bind _returnvalue (`KismetArrayLibrary.Array_Length` _notepool))
  (bind _output (`|GetArrayItem` _notepool (`self.NoteIndex`)))
  (if (> _returnvalue 0)
    (set `self.MaxPool` _returnvalue)
    (`/Engine/EditorBlueprintResources/StandardMacros.IsValid` _output
      (:`Is Valid`
        (`/Game/Notes/BP_Note.ActivateNote` _output)
        (bind _result (`/Engine/EditorBlueprintResources/StandardMacros.IncrementInt` (`self.NoteIndex`))
          (:`  `
            (bind _output_get (set `self.NoteIndex` _result))
            (if (== _output_get (`self.MaxPool`))
              (set `self.NoteIndex` 0))))))))

(fn `SpawnNotes`
  (for _ (range (+ (`self.AmountOfNotes`) 1))
    (bind _returnvalue (`|SpawnActorFromClass` "/Game/Notes/BP_Note.BP_Note_C" (`self.GetTransform`) "Undefined" "MultiplyWithRoot" null null))
    (`PrimitiveComponent.SetCollisionEnabled` (`/Game/Notes/BP_Note.NoteMesh` _returnvalue) "NoCollision")
    (add `/Game/Notes/BP_Note.OnDestruction` _returnvalue (`|CreateDelegate` :!event `OnNoteDestroyed`))
    (`KismetArrayLibrary.Array_Add` (`self.NotePool`) _returnvalue)))

(fn `UserConstructionScript`)