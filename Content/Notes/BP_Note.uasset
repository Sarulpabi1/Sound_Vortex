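; BP_Note is a note pawn that moves toward a random reachable nearby point on BeginPlay and then hides itself.
; A short delay after issuing the AI move, without waiting for arrival, it disables capsule collision and broadcasts OnDestruction.
; A looping TryToSpawn timer also broadcasts OnDestruction with itself.
; The actor is never destroyed here, and ActivateNote can restore visibility and collision, which suggests reuse.
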(event `self.ReceiveBeginPlay`
  (`KismetSystemLibrary.K2_SetTimerDelegate` (delegate `TryToSpawn`) 2.0 true)
  (`self.Movement`))

(event `TryToSpawn`
  (`self.OnDestruction` self))

(event `Movement`
  (`|AIMoveTo` self (`NavigationSystemV1.K2_GetRandomReachablePointInRadius` (`self.K2_GetActorLocation`) 3000.0 null null) null
    (:`then`
      (`KismetSystemLibrary.Delay` 3.0)
      (`self.DesactivateNote`)
      (`self.OnDestruction` null))))

(event `DesactivateNote`
  (`self.SetActorHiddenInGame` true)
  (`PrimitiveComponent.SetCollisionEnabled` (`self.CapsuleComponent`) "NoCollision"))

(event `ActivateNote`
  (`self.SetActorHiddenInGame` false)
  (`PrimitiveComponent.SetCollisionEnabled` (`self.CapsuleComponent`) "QueryAndPhysics"))

(fn `UserConstructionScript`)