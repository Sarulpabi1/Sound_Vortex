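; Note spawner Blueprint that activates notes from a pre-built pool held by a referenced BPNotePool.
; Each Spawn event calls ActivateNote on the pool entry at NoteIndex, then advances the index and wraps to zero at the pool's length, reusing notes round-robin.
; An empty pool or invalid entry activates nothing and leaves the index unchanged.
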(event `Spawn`
  (bind _notepool (`/Game/MapObjects/Notes/BP_NotePool.NotePool` (`self.BP_NotePool`)))
  (bind _returnvalue (`KismetArrayLibrary.Array_Length` _notepool))
  (bind _output (`|GetArrayItem` _notepool (`self.NoteIndex`)))
  (if (> _returnvalue 0)
    (set `self.MaxPool` _returnvalue)
    (`/Engine/EditorBlueprintResources/StandardMacros.IsValid` _output
      (:`Is Valid`
        (`/Game/MapObjects/Notes/BP_Note.ActivateNote` _output)
        (bind _result (`/Engine/EditorBlueprintResources/StandardMacros.IncrementInt` (`self.NoteIndex`))
          (:`  `
            (bind _output_get (set `self.NoteIndex` _result))
            (if (== _output_get (`self.MaxPool`))
              (set `self.NoteIndex` 0))))))))

(fn `UserConstructionScript`)