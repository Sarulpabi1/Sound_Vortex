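; BP_NotePool pre-spawns a pool of BP_Note actors for reuse, parked on the owning actor.
; On BeginPlay it spawns notes at the owner's transform in a count set by AmountOfNotes, disables their mesh collision, attaches them and stores them in NotePool.
; Each note's destruction event is bound to a handler that moves it back to the owner's location and reattaches it.
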(event `self.ReceiveBeginPlay`
  (for _ (range (+ (`self.AmountOfNotes`) 1))
    (bind _returnvalue (`|SpawnActorFromClass` "/Game/MapObjects/Notes/BP_Note.BP_Note_C" (`Actor.GetTransform` (`self.GetOwner`)) "Undefined" "MultiplyWithRoot" null null))
    (`PrimitiveComponent.SetCollisionEnabled` (`/Game/MapObjects/Notes/BP_Note.NoteMesh` _returnvalue) "NoCollision")
    (`Actor.K2_AttachToActor` _returnvalue (`self.GetOwner`) "None" "KeepWorld" "KeepWorld" "KeepWorld" true)
    (add `/Game/MapObjects/Notes/BP_Note.OnDestruction` _returnvalue (delegate `OnNoteDestroyed`))
    (`KismetArrayLibrary.Array_Add` (`self.NotePool`) _returnvalue)))

(event `OnNoteDestroyed`
  (params (Notes :type "/Game/MapObjects/Notes/BP_Note Object Reference"))
  (bind _returnvalue (`self.GetOwner`))
  (`Actor.K2_SetActorLocation` Notes (`Actor.K2_GetActorLocation` _returnvalue) false false)
  (`Actor.K2_AttachToActor` Notes _returnvalue "None" "KeepWorld" "KeepWorld" "KeepWorld" true))