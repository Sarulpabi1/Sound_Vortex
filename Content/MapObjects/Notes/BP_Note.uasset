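; BP_Note is a note map object that hides itself shortly after play begins and signals through its OnDestruction dispatcher.
; BeginPlay starts a looping timer that repeatedly broadcasts OnDestruction, then runs Movement, which waits briefly, deactivates the note and broadcasts again.
; Deactivation hides the actor and disables mesh collision instead of destroying it; ActivateNote reverses this but is not called here.
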(event `self.ReceiveBeginPlay`
  (`KismetSystemLibrary.K2_SetTimerDelegate` (delegate `TryToSpawn`) 2.0 true)
  (`self.Movement`))

(event `TryToSpawn`
  (`self.OnDestruction` self))

(event `Movement`
  (`KismetSystemLibrary.Delay` 3.0)
  (`self.DesactivateNote`)
  (`self.OnDestruction` self))

(event `DesactivateNote`
  (`self.SetActorHiddenInGame` true)
  (`PrimitiveComponent.SetCollisionEnabled` (`self.NoteMesh`) "NoCollision"))

(event `ActivateNote`
  (`self.SetActorHiddenInGame` false)
  (`PrimitiveComponent.SetCollisionEnabled` (`self.NoteMesh`) "QueryAndPhysics"))

(fn `UserConstructionScript`)