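; BP_LignTrigger is a trigger actor that hides BP_Note actors that begin overlapping it while it is active.
; ChangeState sets IsActive and calls TriggerLaunch, which clears the flag after a 0.3-second retriggerable delay, so repeated calls extend the active window.
; The overlap is only checked as it begins, and print strings output the flag as it changes.
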(event `self.ReceiveActorBeginOverlap`
  (params (OtherActor :type "Actor Object Reference"))
  (set `self.MainActor` OtherActor)
  (if (== "/Game/MapObjects/Notes/BP_Note.BP_Note_C" (`GameplayStatics.GetObjectClass` (`self.MainActor`)))
    (if (`self.IsActive`)
      (`self.SetActorHiddenInGame` (`self.MainActor`) true))))

(event `TriggerLaunch`
  (bind _isactive (`self.IsActive`))
  (bind _returnvalue (`KismetStringLibrary.Conv_BoolToString` _isactive))
  (if _isactive
    (`KismetSystemLibrary.PrintString` _returnvalue)
    (`KismetSystemLibrary.RetriggerableDelay` 0.3)
    (set `self.IsActive` false)
    (`KismetSystemLibrary.PrintString` _returnvalue)))

(fn `ChangeState`
  (`KismetSystemLibrary.PrintString` (`KismetStringLibrary.Conv_BoolToString` (`self.IsActive`)))
  (set `self.IsActive` true)
  (`self.TriggerLaunch`))

(fn `UserConstructionScript`)