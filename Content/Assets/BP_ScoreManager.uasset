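; BP_ScoreManager is an actor that pushes the current score to the on-screen UI.
; On BeginPlay it finds the BP_Controller actor and caches it, along with an unused reference to its BPUI widget.
; An UpdateScore event converts the Score variable to text and writes it into TextBlock1 of the controller's widget.
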(event `self.ReceiveBeginPlay`
  (bind _returnvalue (`GameplayStatics.GetActorOfClass` "/Game/Systems/BP_Controller.BP_Controller_C"))
  (set `self.BPController` _returnvalue)
  (set `self.WidgetUser` (`/Game/Systems/BP_Controller.BPUI` (`self.BPController`)))
  (`GameplayStatics.GetActorOfClass` "BP_ScoreManager_C"))

(event `UpdateScore`
  (set `TextBlock.Text` (`KismetTextLibrary.Conv_IntToText` (`self.Score`)) (`/Game/Assets/UI/BP_UI.TextBlock_1` (`/Game/Systems/BP_Controller.BPUI` (`self.BPController`)))))

(fn `UserConstructionScript`)