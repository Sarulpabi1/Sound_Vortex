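; BP_Controller handles player input and UI, driving four column triggers and a toggleable user menu.
; On BeginPlay it adds the Enhanced Input mapping context, caches all LignTrigger actors and creates both widgets, showing BP_UI only on MapLevel1.
; The four column actions call ChangeState on cached triggers by array index, so key-to-column mapping depends on GetAllActorsOfClass order.
; The menu action toggles BP_UserMenu visibility through IsShown.
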(event `self.ReceiveBeginPlay`
  (bind _bpui (`self.BPUI`))
  (`EnhancedInputSubsystemInterface.AddMappingContext` (subsystem `EnhancedInputLocalPlayerSubsystem`) "/Game/Inputs/IMC_InputActionMap.IMC_InputActionMap" 0 (struct))
  (bind _outactors (`GameplayStatics.GetAllActorsOfClass` "/Game/Assets/LignTrigger.LignTrigger_C"))
  (set `self.LignActors` _outactors)
  (bind _returnvalue (`|CreateWidget` "/Game/Assets/UI/BP_UI.BP_UI_C"))
  (set `self.BPUI` _returnvalue)
  (`UserWidget.AddToViewport` (`self.BPUI`) 0)
  (bind _returnvalue_2 (`|CreateWidget` "/Game/Assets/UI/BP_UserMenu.BP_UserMenu_C"))
  (bind _output_get (set `self.BPUserMenu` _returnvalue_2))
  (`UserWidget.AddToViewport` _output_get 0)
  (set `Widget.Visibility` "Hidden" (`self.BPUserMenu`))
  (if (== (`self.MapLevel1`) (`self.GetLevel`))
    (set `Widget.Visibility` "Visible" _bpui)
    (else
      (set `Widget.Visibility` "Hidden" _bpui))))

(event `EnhancedInput|/Game/Inputs/IA_ActivateColumns/IA_ActivateColumn1`
  (params (ActionValue :type Boolean) (ElapsedSeconds :type "Float (double-precision)") (TriggeredSeconds :type "Float (double-precision)") (InputAction :type "InputAction Object Reference" :default "/Game/Inputs/IA_ActivateColumns/IA_ActivateColumn1.IA_ActivateColumn1"))
  (:`Triggered`
    (`/Game/Assets/LignTrigger.ChangeState` (`|GetArrayItem` (`self.LignActors`)))))

(event `EnhancedInput|/Game/Inputs/IA_ActivateColumns/IA_ActivateColumn2`
  (params (ActionValue :type Boolean) (ElapsedSeconds :type "Float (double-precision)") (TriggeredSeconds :type "Float (double-precision)") (InputAction :type "InputAction Object Reference" :default "/Game/Inputs/IA_ActivateColumns/IA_ActivateColumn2.IA_ActivateColumn2"))
  (:`Triggered`
    (`/Game/Assets/LignTrigger.ChangeState` (`|GetArrayItem` (`self.LignActors`) 1))))

(event `EnhancedInput|/Game/Inputs/IA_ActivateColumns/IA_ActivateColumn3`
  (params (ActionValue :type Boolean) (ElapsedSeconds :type "Float (double-precision)") (TriggeredSeconds :type "Float (double-precision)") (InputAction :type "InputAction Object Reference" :default "/Game/Inputs/IA_ActivateColumns/IA_ActivateColumn3.IA_ActivateColumn3"))
  (:`Triggered`
    (`/Game/Assets/LignTrigger.ChangeState` (`|GetArrayItem` (`self.LignActors`) 2))))

(event `EnhancedInput|/Game/Inputs/IA_ActivateColumns/IA_ActivateColumn4`
  (params (ActionValue :type Boolean) (ElapsedSeconds :type "Float (double-precision)") (TriggeredSeconds :type "Float (double-precision)") (InputAction :type "InputAction Object Reference" :default "/Game/Inputs/IA_ActivateColumns/IA_ActivateColumn4.IA_ActivateColumn4"))
  (:`Triggered`
    (`/Game/Assets/LignTrigger.ChangeState` (`|GetArrayItem` (`self.LignActors`) 3))))

(event `EnhancedInput|/Game/Inputs/IA_ActivateMenu`
  (params (ActionValue :type Boolean) (ElapsedSeconds :type "Float (double-precision)") (TriggeredSeconds :type "Float (double-precision)") (InputAction :type "InputAction Object Reference" :default "/Game/Inputs/IA_ActivateMenu.IA_ActivateMenu"))
  (bind _bpusermenu (`self.BPUserMenu`))
  (:`Triggered`
    (if (`self.IsShown`)
      (set `Widget.Visibility` "Hidden" _bpusermenu)
      (set `self.IsShown` false)
      (else
        (set `Widget.Visibility` "Visible" _bpusermenu)
        (set `self.IsShown` true)))))

(fn `UserConstructionScript`)