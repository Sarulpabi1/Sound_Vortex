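; BP_Gamemode is a game mode that hands out a pool of notes to BP_Spawner actors.
; Start sets the remaining-note count from the summed NotePool map values, then queues one note per pool entry on a randomly picked spawner.
; GetSpawners caches the level's spawners, but nothing here calls it or Start.
; GetNoteFromPool only returns the Notes variable without drawing from the pool, and End is empty.
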(fn `BuildNotePool`
  (locals (LocalSum :type Integer))
  (set `self.NotesRemaining` (`self.GetPoolSize`)))

(fn `End`)

(fn `GetNoteFromPool`
  (returns (Note :type "/Game/Notes/Notes Class Reference"))
  (return "/Game/Notes/Notes.Notes_C"))

(fn `GetPoolSize`
  (returns (LocalSum1 :type Integer))
  (locals (LocalSum :type Integer))
  (bind _values (`BlueprintMapLibrary.Map_Values` (`self.NotePool`)))
  (for _array_element _values
    (set `local.LocalSum` (+ _array_element (`local.LocalSum`))))
  (return (`local.LocalSum`)))

(fn `GetSpawners`
  (bind _outactors (`GameplayStatics.GetAllActorsOfClass` "/Game/Notes/BP_Spawner.BP_Spawner_C"))
  (set `self.Spawners` _outactors))

(fn `Start`
  (`self.BuildNotePool`)
  (for _ (range (`self.GetPoolSize`))
    (bind _note (`self.GetNoteFromPool`))
    (`/Game/Notes/BP_Spawner.AddToQueue` (`KismetArrayLibrary.Array_Random` (`self.Spawners`)) _note)))

(fn `UserConstructionScript`)